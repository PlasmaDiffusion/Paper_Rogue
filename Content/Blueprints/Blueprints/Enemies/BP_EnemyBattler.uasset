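; Enemy battler for turn-based combat that tracks HP on a text and scaled bar and attacks allies by moving into them.
; PickCommand rolls an ability, but PickTarget ignores it, always resolving to front-row allies because its random back-row check never succeeds.
; Tick lerps toward the target; box overlap deals Atk damage if the row matches TargetPlayer, then sends it home to end the turn via Pawn_BattleHandler.
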(event OnComponentBeginOverlap(Box)
  (params (OverlappedComponent :type Primitive%20Component%20Object%20Reference) (OtherActor :type Actor%20Object%20Reference) (OtherComp :type Primitive%20Component%20Object%20Reference) (OtherBodyIndex :type Integer) (bFromSweep :type Boolean) (SweepResult :type Hit%20Result%20Structure%20%28by%20ref%29))
  ;[1 1 1] Attack! (But only if it's the right target and the enemy didn't already attack.
  (if (not (Variables|movement|Getattacked))
    (bind _asbp_ally_battler (Utilities|Casting|CastToBP_AllyBattler OtherActor))
    (if (Math|Boolean|Equal(Boolean) (Variables|/Game/Blueprints/Blueprints/Character/BP_AllyBattler.BP_AllyBattler_C|GetfrontRow _asbp_ally_battler) (Math|Conversions|ToBoolean(Integer) (Variables|movement|GettargetPlayer)))
      (Default|TakeDamage _asbp_ally_battler (Variables|Default|GetAtk))
      ;[1 1 1] After attack go back to original position
      (Variables|movement|SetgoToTargetPos true)
      (Variables|movement|SettargetAlpha 0.0)
      (Variables|movement|Setattacked true)
      (Variables|movement|SettargetPos (Variables|movement|GetoriginalPos)))))

(event EventBeginPlay
  (Variables|Default|SetmaxHP (Variables|Default|GetHP))
  (Variables|movement|SetoriginalPos (Transformation|GetActorLocation))
  (CallFunction|UpdateHPBar))

(event EventTick
  (params (DeltaSeconds :type Float%20%28single-precision%29))
  ;[1 1 1] Move towards target
  (if (Variables|movement|GetgoToTargetPos)
    (bind _output_get (Variables|movement|SettargetAlpha (+ (Variables|movement|GettargetAlpha) (* DeltaSeconds 0.2))))
    (Transformation|SetActorLocation (Math|Vector|Lerp(Vector) (Transformation|GetActorLocation) (Variables|movement|GettargetPos) _output_get) false false)
    ;[1 1 1] If back at original spot after attacking end turn
    (if (Math|Boolean|ANDBoolean (Math|Vector|Equal(Vector) (Transformation|GetActorLocation) (Variables|movement|GetoriginalPos) 5e-05) (Variables|movement|Getattacked) true)
      (bind _outactors (Actor|GetAllActorsOfClass "/Game/Blueprints/Blueprints/Character/Pawn_BattleHandler.Pawn_BattleHandler_C"))
      (Default|EndEnemyTurn (Utilities|Array|Get(acopy) _outactors))
      (Variables|movement|Setattacked false)
      (Variables|movement|SetgoToTargetPos false)
      (Variables|movement|SettargetAlpha 0.0)
      (Development|PrintString "enemy ended turn")
      (Rendering|SetVisibility (Variables|Default|GetPaperSprite1) true true))))

(fn ConstructionScript)

(fn PickCommand
  (LocalVariables|SetrandomInt (Math|Random|RandomIntegerinRange 1 100))
  (bind _array_element (Utilities|Array|ForEachLoopwithBreak (Variables|Default|GetCommands) :!label _label)
    (:LoopBody
      (if (and (>= (LocalVariables|GetrandomInt) (.chanceMin (Utilities|Struct|BreakSt_EnemyAbilityAI _array_element))) (<= 0 (.chanceMax (Utilities|Struct|BreakSt_EnemyAbilityAI _array_element))))
        (LocalVariables|SetnewAttack (.abilityName (Utilities|Struct|BreakSt_EnemyAbilityAI _array_element)))
        (goto _label Break)))
    (:Completed
      (CallFunction|PickTarget (LocalVariables|GetnewAttack)))))

(fn PickTarget
  (params (attackName :type String))
  (LocalVariables|SettargettingFrontPlayer (not (== (Math|Random|RandomInteger 3) 3)))
  (bind _outactors (Actor|GetAllActorsOfClass "/Game/Blueprints/Blueprints/Character/BP_AllyBattler.BP_AllyBattler_C"))
  ;[1 1 1] See which player is in the front row and get their position (Only applies to attacks with target value of 1)
  (for _array_element _outactors
    (if (Math|Boolean|Equal(Boolean) (Variables|/Game/Blueprints/Blueprints/Character/BP_AllyBattler.BP_AllyBattler_C|GetfrontRow _array_element) (LocalVariables|GettargettingFrontPlayer))
      (Variables|movement|SettargetPos (Transformation|GetActorLocation _array_element))
      (Variables|movement|SetgoToTargetPos true)
      (Default|ActivateGuarding _array_element)
      (Rendering|SetVisibility (Variables|Default|GetPaperSprite1) false true))))

(fn UpdateHPBar
  (Rendering|Components|TextRender|SetText (Variables|Default|GetHP_Text) (Utilities|Text|ToText(Integer) (Variables|Default|GetHP)))
  (Transformation|SetRelativeScale3D (Variables|Default|GetHP_Bar) (Math|Vector|MakeVector (/ (Math|Conversions|ToFloat(Integer) (Variables|Default|GetHP)) (Math|Conversions|ToFloat(Integer) (Variables|Default|GetmaxHP))) 1.0 1.0)))