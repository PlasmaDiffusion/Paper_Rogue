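; BP_splashDamage is a short-lived visual effect actor, likely a splash damage indicator, made of a TextRender and a Plane.
; Tick runs through a short Delay, so each step fires at a throttled interval rather than every frame.
; Each step enlarges the text and spins the plane, and the actor destroys itself once the text reaches its size limit.
; It contains no damage logic.
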(event EventBeginPlay)

(event Collision|EventActorBeginOverlap
  (params (OtherActor :type Actor%20Object%20Reference)))

(event EventTick
  (params (DeltaSeconds :type Float%20%28single-precision%29))
  (Utilities|FlowControl|Delay 0.05)
  (Transformation|SetRelativeScale3D (Variables|Default|GetTextRender) (+ (Variables|/Script/Engine.SceneComponent|GetRelativeScale3D (Variables|Default|GetTextRender)) "0.250000,0.250000,0.250000"))
  (if (>= (.X (Math|Vector|BreakVector (Variables|/Script/Engine.SceneComponent|GetRelativeScale3D (Variables|Default|GetTextRender)))) 4.0)
    (Actor|DestroyActor)
    (else
      (Transformation|AddLocalRotation (Variables|Default|GetPlane) "0.000000,5.000000,0.000000" false false))))

(fn ConstructionScript)