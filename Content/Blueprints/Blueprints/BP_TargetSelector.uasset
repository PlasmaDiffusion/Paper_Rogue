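; Battle target-selector actor that hovers above the enemy currently targeted in a Pawn_BattleHandler fight.
; In enemy-select mode, Tick reads the handler's left/right input and Move steps its SelectedTarget index with wraparound, calling MoveOverEnemyTarget on wrap.
; ForceOntoFrontTarget snaps above the selected index if any enemy is alive.
; Ally selection is unfinished: its Tick branch is empty and MoveOverPlayerTarget is never called here.
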(event EventBeginPlay
  (bind _outactors (Actor|GetAllActorsOfClass "/Game/Blueprints/Blueprints/Character/Pawn_BattleHandler.Pawn_BattleHandler_C"))
  (Utilities|Casting|CastToPawn_BattleHandler (Utilities|Array|Get(acopy) _outactors))
  (Variables|Default|SetbattleHandler 0))

(event Collision|EventActorBeginOverlap
  (params (OtherActor :type Actor%20Object%20Reference)))

(event EventTick
  (params (DeltaSeconds :type Float%20%28single-precision%29))
  (bind _battlehandler (Variables|Default|GetbattleHandler))
  (if (== (Variables|Default|Gettype) 1) ; See if selecting enemy
    ;[1 1 1] Move target onto enemy
    (if (Variables|/Game/Blueprints/Blueprints/Character/Pawn_BattleHandler.Pawn_BattleHandler_C|GetinputRight _battlehandler)
      (CallFunction|Move true)
      (elif (Variables|/Game/Blueprints/Blueprints/Character/Pawn_BattleHandler.Pawn_BattleHandler_C|GetinputLeft _battlehandler)
        (CallFunction|Move false)))
    (elif (== (Class|KismetMathLibrary|OrIntInt 4 5) (Variables|Default|Gettype)) ; See if selecting ally
      _)))

(fn ConstructionScript)

(fn Move
  (params (right :type Boolean))
  (bind _battlehandler (Variables|Default|GetbattleHandler))
  (bind _enemeies (Variables|/Game/Blueprints/Blueprints/Character/Pawn_BattleHandler.Pawn_BattleHandler_C|Getenemeies _battlehandler))
  (bind _returnvalue (Utilities|Array|Length _enemeies))
  (if right
    (bind _result (Math|Integer|IncrementInt (Variables|/Game/Blueprints/Blueprints/Character/Pawn_BattleHandler.Pawn_BattleHandler_C|GetselectedTarget _battlehandler)) ; Increment. If > array size then make equal to zero
      (:%20%20
        (if (> _result _returnvalue)
          (Variables|/Game/Blueprints/Blueprints/Character/Pawn_BattleHandler.Pawn_BattleHandler_C|SetselectedTarget (Variables|Default|GetbattleHandler) 0)
          (CallFunction|MoveOverEnemyTarget :!label _label))))
    (else
      (bind _result_2 (Math|Integer|DecrementInt (Variables|/Game/Blueprints/Blueprints/Character/Pawn_BattleHandler.Pawn_BattleHandler_C|GetselectedTarget _battlehandler)) ; Decrement. If < 0 then make equal to array size
        (:%20%20
          (if (<= _result_2 0)
            (Variables|/Game/Blueprints/Blueprints/Character/Pawn_BattleHandler.Pawn_BattleHandler_C|SetselectedTarget (Variables|Default|GetbattleHandler) (- _returnvalue 1))
            (goto _label)))))))

(fn MoveOverEnemyTarget
  (bind _battlehandler (Variables|Default|GetbattleHandler))
  (Transformation|SetActorLocation (+ (Transformation|GetActorLocation (Utilities|Array|Get(acopy) (Variables|/Game/Blueprints/Blueprints/Character/Pawn_BattleHandler.Pawn_BattleHandler_C|Getenemeies _battlehandler) (Variables|/Game/Blueprints/Blueprints/Character/Pawn_BattleHandler.Pawn_BattleHandler_C|GetselectedTarget _battlehandler))) "0, 0,100.000000") false false))

(fn MoveOverPlayerTarget
  (bind _battlehandler (Variables|Default|GetbattleHandler))
  (Transformation|SetActorLocation (+ (Transformation|GetActorLocation (Utilities|Array|Get(acopy) (Variables|/Game/Blueprints/Blueprints/Character/Pawn_BattleHandler.Pawn_BattleHandler_C|Getallies _battlehandler) (Variables|/Game/Blueprints/Blueprints/Character/Pawn_BattleHandler.Pawn_BattleHandler_C|GetselectedTarget _battlehandler))) "0, 0,100.000000") false false))

(fn ForceOntoFrontTarget
  (bind _battlehandler (Variables|Default|GetbattleHandler))
  (bind _enemeies (Variables|/Game/Blueprints/Blueprints/Character/Pawn_BattleHandler.Pawn_BattleHandler_C|Getenemeies _battlehandler))
  (bind _array_element (Utilities|Array|ForEachLoopwithBreak _enemeies :!label _label)
    (:LoopBody
      (if (Variables|/Game/Blueprints/Blueprints/Enemies/BP_EnemyBattler.BP_EnemyBattler_C|Getalive _array_element)
        (Transformation|SetActorLocation (+ (Transformation|GetActorLocation (Utilities|Array|Get(acopy) _enemeies (Variables|/Game/Blueprints/Blueprints/Character/Pawn_BattleHandler.Pawn_BattleHandler_C|GetselectedTarget _battlehandler))) "0, 0,100.000000") false false)
        (goto _label Break)))))