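; BP_ActionCommand is a short-lived button-mashing action command for the player's attack in battle.
; While its timer counts down on Tick, it polls InputB on Pawn_BattleHandler, counting presses, playing a sound and nudging a sphere sideways for each.
; At timeout it rates the press count as one of two tiers, passes that rating to the handler's PlayerAttacking, and destroys itself.
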(event EventBeginPlay
  (bind _outactors (Actor|GetAllActorsOfClass "/Game/Blueprints/Blueprints/Character/Pawn_BattleHandler.Pawn_BattleHandler_C"))
  (Variables|Default|SetplayerBattlerActor (Utilities|Array|Get(acopy) _outactors)))

(event Collision|EventActorBeginOverlap
  (params (OtherActor :type Actor%20Object%20Reference)))

(event EventTick
  (params (DeltaSeconds :type Float%20%28single-precision%29))
  (bind _sphere (Variables|Default|GetSphere))
  (bind _output_get (Variables|Default|Settimer (- (Variables|Default|Gettimer) DeltaSeconds)))
  (if (< _output_get 0.0)
    (if (>= (Variables|Default|Getpresses) 10)
      (Variables|Default|Setrating 2)
      (Audio|PlaySound2D "/Game/StarterContent/Audio/Explosion01.Explosion01" 0.3)
      (else
        (Variables|Default|Setrating 1)))
    (bind _outactors (Actor|GetAllActorsOfClass "/Game/Blueprints/Blueprints/Character/Pawn_BattleHandler.Pawn_BattleHandler_C"))
    (Default|PlayerAttacking (Utilities|Array|Get(acopy) _outactors) 0 "" 0 0 (Variables|Default|Getrating))
    (Actor|DestroyActor)
    (else
      ;[1 1 1] Mash X!
      (if (Variables|/Game/Blueprints/Blueprints/Character/Pawn_BattleHandler.Pawn_BattleHandler_C|GetinputB (Variables|Default|GetplayerBattlerActor))
        (Math|Integer|IncrementInt (Variables|Default|Getpresses)
          (:%20%20
            (Audio|PlaySound2D "/Game/StarterContent/Audio/Collapse02.Collapse02" 0.5 1.0 3.0)
            (Transformation|SetRelativeLocation _sphere (+ (Variables|/Script/Engine.SceneComponent|GetRelativeLocation _sphere) "0.000000,-40.000000, 0") false false)))))))

(fn ConstructionScript)