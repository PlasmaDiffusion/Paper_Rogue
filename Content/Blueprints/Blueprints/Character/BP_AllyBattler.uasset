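; BP_AllyBattler is the player-side battler that handles timed guarding and incoming damage in battle.
; While guarding is enabled, Tick reads InputA from Pawn_BattleHandler to open a brief guard window, followed by a short lockout before re-guarding.
; TakeDamage subtracts guard and, for the non-partner, Defense, writes HP to the partner or player data in RPG_GameMode, then spawns floating damage text.
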(event OnComponentBeginOverlap(Box)
  (params (OverlappedComponent :type Primitive%20Component%20Object%20Reference) (OtherActor :type Actor%20Object%20Reference) (OtherComp :type Primitive%20Component%20Object%20Reference) (OtherBodyIndex :type Integer) (bFromSweep :type Boolean) (SweepResult :type Hit%20Result%20Structure%20%28by%20ref%29)))

(event EventBeginPlay
  (bind _outactors (Actor|GetAllActorsOfClass "/Game/Blueprints/Blueprints/Character/Pawn_BattleHandler.Pawn_BattleHandler_C"))
  (Variables|Default|SetbattleManager (Utilities|Array|Get(acopy) _outactors)))

(event Collision|EventActorBeginOverlap
  (params (OtherActor :type Actor%20Object%20Reference)))

(event EventTick
  (params (DeltaSeconds :type Float%20%28single-precision%29))
  ;[1 1 1] Check if being attacked...
  (if (Variables|Default|GetcanGuard)
    ;[1 1 1] Can only guard for a limited time...
    (Variables|Default|SetguardTime (- (Variables|Default|GetguardTime) DeltaSeconds))
    ;[1 1 1] Determine if guard timed out
    (if (and (< (Variables|Default|GetguardTime) 0.25) (> (Variables|Default|GetguardTime) 0.0))
      (Variables|Default|Setguarding false)
      (Rendering|SetVisibility (Variables|Default|GetGuardSprite) false false)
      (Development|PrintString "guard off")
      (else
        ;[1 1 1] Start guarding if A is pressed
        (if (Variables|/Game/Blueprints/Blueprints/Character/Pawn_BattleHandler.Pawn_BattleHandler_C|GetinputA (Variables|Default|GetbattleManager))
          (if (and (not (Variables|Default|Getguarding)) (<= (Variables|Default|GetguardTime) 0.0))
            (Variables|Default|Setguarding true)
            (Variables|Default|SetguardTime (Variables|Default|GetguardTimeMax))
            (Rendering|SetVisibility (Variables|Default|GetGuardSprite) true false)
            (Development|PrintString "guard on")))))))

(fn ConstructionScript)

(fn TakeDamage
  (params (damage :type Integer) (element :type Integer) (statusEffect :type Integer))
  (Rendering|SetVisibility (Variables|Default|GetGuardSprite) false false)
  (Variables|Default|SetcanGuard false)
  (LocalVariables|Setdmg damage)
  (LocalVariables|Setelm element)
  (bind _asrpg_game_mode (Utilities|Casting|CastToRPG_GameMode (Game|GetGameMode)))
  (LocalVariables|SetgameMode _asrpg_game_mode)
  (if (Variables|Default|GetisPartner)
    (bind (_newhp _outputdamage) (CallFunction|CalculateDamage (LocalVariables|Getdmg) (LocalVariables|Getelm) (.HP (Utilities|Struct|BreakSt_Partners (Utilities|Array|Get(acopy) (Variables|/Game/Blueprints/Blueprints/RPG_GameMode.RPG_GameMode_C|GetpartnersInParty (LocalVariables|GetgameMode)) (Variables|/Game/Blueprints/Blueprints/RPG_GameMode.RPG_GameMode_C|GetcurrentPartner (LocalVariables|GetgameMode))))) 0 false))
    (|SetBy-RefVar (.HP (Utilities|Struct|BreakSt_Partners (Utilities|Array|Get(acopy) (Variables|/Game/Blueprints/Blueprints/RPG_GameMode.RPG_GameMode_C|GetpartnersInParty (LocalVariables|GetgameMode)) (Variables|/Game/Blueprints/Blueprints/RPG_GameMode.RPG_GameMode_C|GetcurrentPartner (LocalVariables|GetgameMode))))) _newhp)
    (LocalVariables|Setoutput _outputdamage)
    (else
      (bind (_newhp_2 _outputdamage_2) (CallFunction|CalculateDamage (LocalVariables|Getdmg) (LocalVariables|Getelm) (Variables|/Game/Blueprints/Blueprints/RPG_GameMode.RPG_GameMode_C|GetHP (LocalVariables|GetgameMode)) (Variables|/Game/Blueprints/Blueprints/RPG_GameMode.RPG_GameMode_C|Getdefense (LocalVariables|GetgameMode)) false))
      (LocalVariables|Setoutput _outputdamage_2)
      (Variables|/Game/Blueprints/Blueprints/RPG_GameMode.RPG_GameMode_C|SetHP (LocalVariables|GetgameMode) _newhp_2)))
  ;[1 1 1] Output damage text
  (bind _returnvalue (Game|SpawnActorfromClass "/Game/Blueprints/Blueprints/BP_splashDamage.BP_splashDamage_C" (Math|Transform|MakeTransform (+ (Transformation|GetActorLocation) "10.000000,10.000000,100.000000") "0, 0, 0" "2.000000,2.000000,2.000000") "Undefined" 0 0))
  (Rendering|Components|TextRender|SetText (Variables|/Game/Blueprints/Blueprints/BP_splashDamage.BP_splashDamage_C|GetTextRender _returnvalue) (Utilities|Text|ToText(Integer) (LocalVariables|Getoutput))))

(fn CalculateDamage
  (params (dmg :type Integer) (element :type Integer) (HP_toLower :type Integer) (Defense :type Integer) (enemyBeingDamgaged :type Boolean))
  (bind _guarding (Variables|Default|Getguarding))
  (bind _returnvalue (Math|Conversions|ToInteger(Boolean) _guarding))
  (bind _returnvalue_2 (- dmg _returnvalue))
  (bind _returnvalue_3 (- _returnvalue_2 Defense))
  (bind _returnvalue_4 (Math|Integer|Clamp(Integer) _returnvalue_3 0 99))
  (return (- HP_toLower _returnvalue_4) _returnvalue_4))

(fn ActivateGuarding
  (Variables|Default|SetguardTime 0.0)
  (Variables|Default|SetcanGuard true)
  (Variables|Default|Setguarding false)
  (Rendering|SetVisibility (Variables|Default|GetGuardSprite) false false))