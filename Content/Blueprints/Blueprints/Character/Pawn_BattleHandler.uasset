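; Player-possessed pawn that runs a turn-based RPG battle between player, partner and enemies.
; Tick drives a mode state machine: command menus, target selection, enemy turns and turn end, with throttled directional input.
; Billboard and text components form the menus, filled with badge or partner attacks from RPG_GameMode.
; Confirming a target spawns an action-command actor; PlayerAttacking applies its rating as damage, spends MP and advances the turn.
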(event EventBeginPlay
  (bind _returnvalue (Game|GetPlayerController 0))
  ;[1 1 1] Switch to battle pawn
  (Pawn|UnPossess _returnvalue)
  (Pawn|Possess _returnvalue self)
  ;[1 1 1] Component arrays
  (Variables|Default|SetcommandGroupBillboards (Utilities|Array|MakeArray (Variables|Default|GetBillboard) (Variables|Default|GetBillboard1) (Variables|Default|GetBillboard2)))
  (Variables|Default|SetcommandTexts (Utilities|Array|MakeArray (Variables|Default|GetsubmenuCommand) (Variables|Default|GetsubmenuCommand1) (Variables|Default|GetsubmenuCommand2) (Variables|Default|GetsubmenuCommand3) (Variables|Default|GetsubmenuCommand4)))
  (bind _outactors (Actor|GetAllActorsOfClass "/Game/Blueprints/Blueprints/Enemies/BP_EnemyBattler.BP_EnemyBattler_C"))
  (Variables|enemies|Setenemeies _outactors)
  (bind _asrpg_game_mode (Utilities|Casting|CastToRPG_GameMode (Game|GetGameMode)))
  (Variables|Default|SetgameMode _asrpg_game_mode))

(event Collision|EventActorBeginOverlap
  (params (OtherActor :type Actor%20Object%20Reference)))

(event EventTick
  (params (DeltaSeconds :type Float%20%28single-precision%29))
  (if (Variables|Default|GetbriefDelay) ; Brief delay for end of actions
    (Utilities|FlowControl|Delay 0.5)
    (Variables|Default|SetbriefDelay false))
  (switch Utilities|FlowControl|Switch|SwitchonBattleMode (Variables|Default|Getmode)
    (:NewEnumerator0
      (commands|PlayerTurn)
      (CallFunction|InputLag DeltaSeconds :!label _label)
      (Variables|Input|SetinputA false)
      (Variables|Input|SetinputB false))
    (:NewEnumerator2
      (enemies|StartEnemyTurn))
    (:NewEnumerator4
      (Targets|SelectTarget)
      (goto _label))
    (:NewEnumerator3
      (CallFunction|EndTurn))))

(event Input|GamepadEvents|GamepadLeftStickRight
  (params (Key :type Key%20Structure))
  ;[1 1 1] Thumbstick Directions
  (:Pressed
    (Variables|Input|SetinputRight true))
  (:Released
    (Variables|Input|SetinputRight false)))

(event Input|GamepadEvents|GamepadLeftStickUp
  (params (Key :type Key%20Structure))
  ;[1 1 1] Thumbstick Directions
  (:Pressed
    (Variables|Input|SetinputUp true))
  (:Released
    (Variables|Input|SetinputUp false)))

(event Input|GamepadEvents|GamepadLeftStickDown
  (params (Key :type Key%20Structure))
  ;[1 1 1] Thumbstick Directions
  (:Pressed
    (Variables|Input|SetinputDown true))
  (:Released
    (Variables|Input|SetinputDown false)))

(event Input|GamepadEvents|GamepadLeftStickLeft
  (params (Key :type Key%20Structure))
  ;[1 1 1] Thumbstick Directions
  (:Pressed
    (Variables|Input|SetinputLeft true))
  (:Released
    (Variables|Input|SetinputLeft false)))

(event Input|KeyboardEvents|Z
  (params (Key :type Key%20Structure))
  ;[1 1 1] Face Buttons
  (:Released
    (Variables|Input|SetinputB true)))

(event Input|KeyboardEvents|X
  (params (Key :type Key%20Structure))
  ;[1 1 1] Face Buttons
  (:Released
    (Variables|Input|SetinputA true)))

(event Input|GamepadEvents|GamepadFaceButtonBottom
  (params (Key :type Key%20Structure))
  ;[1 1 1] Face Buttons
  (:Released
    (Variables|Input|SetinputA true)))

(event Input|GamepadEvents|GamepadFaceButtonLeft
  (params (Key :type Key%20Structure))
  ;[1 1 1] Face Buttons
  (:Released
    (Variables|Input|SetinputB true)))

(event Input|KeyboardEvents|Left
  (params (Key :type Key%20Structure))
  ;[1 1 1] Arrow Keys
  (:Pressed
    (Variables|Input|SetinputLeft true))
  (:Released
    (Variables|Input|SetinputLeft false)))

(event Input|KeyboardEvents|Right
  (params (Key :type Key%20Structure))
  ;[1 1 1] Arrow Keys
  (:Pressed
    (Variables|Input|SetinputRight true))
  (:Released
    (Variables|Input|SetinputRight false)))

(event Input|KeyboardEvents|Up
  (params (Key :type Key%20Structure))
  ;[1 1 1] Arrow Keys
  (:Pressed
    (Variables|Input|SetinputUp true))
  (:Released
    (Variables|Input|SetinputUp false)))

(event Input|KeyboardEvents|Down
  (params (Key :type Key%20Structure))
  ;[1 1 1] Arrow Keys
  (:Pressed
    (Variables|Input|SetinputDown true))
  (:Released
    (Variables|Input|SetinputDown false)))

(fn ConstructionScript)

(fn PlayerTurn
  (if (Variables|Default|GetinSubMenu) ; If not in submenu then...
    ;[1 1 1] Command selection
    (if (Variables|Input|GetinputUp)
      (Math|Integer|DecrementInt (Variables|Default|GetcommandSelected)
        (:%20%20
          (Variables|Default|SetcommandSelected (Math|Integer|Clamp(Integer) (Variables|Default|GetcommandSelected) 0 (- (Utilities|Array|Length (Variables|Default|GetcommandTexts)) 1)) :!label _label)
          ;[1 1 1] Highlight selected command text
          (for (_array_element _array_index) (Variables|Default|GetcommandTexts)
            (if (== _array_index (Variables|Default|GetcommandSelected))
              (Rendering|Components|TextRender|SetTextRenderColor _array_element (Math|Color|MakeColor 0 0 255 255))
              (else
                (Rendering|Components|TextRender|SetTextRenderColor _array_element (Math|Color|MakeColor 255 255 0 255)))))))
      (elif (Variables|Input|GetinputDown)
        (Math|Integer|IncrementInt (Variables|Default|GetcommandSelected)
          (:%20%20
            (goto _label)))
        (else
          ;[1 1 1] Press A to select command and proceed to select target
          (if (Variables|Input|GetinputA)
            (Variables|Default|Setmode "NewEnumerator4")
            ;[1 1 1] Search for attack in database, then check if player has enough MP.
            (if (.ReturnValue (Utilities|Map|Find (Variables|/Game/Blueprints/Blueprints/RPG_GameMode.RPG_GameMode_C|GetDB_PlayerAbilities (Variables|Default|GetgameMode)) (Utilities|String|ToString(Text) (Variables|/Script/Engine.TextRenderComponent|GetText (Utilities|Array|Get(acopy) (Variables|Default|GetcommandTexts) (Variables|Default|GetcommandSelected))))))
              (bind _output_get (Variables|Default|SetcurrentPlayerAttack (.Value (Utilities|Map|Find (Variables|/Game/Blueprints/Blueprints/RPG_GameMode.RPG_GameMode_C|GetDB_PlayerAbilities (Variables|Default|GetgameMode)) (Utilities|String|ToString(Text) (Variables|/Script/Engine.TextRenderComponent|GetText (Utilities|Array|Get(acopy) (Variables|Default|GetcommandTexts) (Variables|Default|GetcommandSelected))))))))
              (if (>= (Variables|/Game/Blueprints/Blueprints/RPG_GameMode.RPG_GameMode_C|GetMP (Variables|Default|GetgameMode)) (.mpCost (Utilities|Struct|BreakSt_AttacksAndAbilities _output_get)))
                (commands|ToggleSubmenuText)
                (Targets|CreateTarget (.targets (Utilities|Struct|BreakSt_AttacksAndAbilities _output_get)))))
            (else
              ;[1 1 1] Back out
              (if (Variables|Input|GetinputB)
                (Variables|Default|SetinSubMenu false)
                (commands|ToggleSubmenuText)
                (commands|ToggleGroupBillboards)))))))
    (else
      ;[1 1 1] Command group selection (attack, item, tactics)
      (if (Variables|Input|GetinputLeft)
        (Math|Integer|DecrementInt (Variables|Default|GetplayerCommandGroup)
          (:%20%20
            ;[1 1 1] Clamp command group
            (bind _output_get_2 (Variables|Default|SetplayerCommandGroup (Math|Integer|Clamp(Integer) (Variables|Default|GetplayerCommandGroup) 0 2) :!label _label_2))
            ;[1 1 1] Highlight selected command group
            (for (_array_element_2 _array_index_2) (Variables|Default|GetcommandGroupBillboards)
              (if (== _array_index_2 _output_get_2)
                (LocalVariables|SetnewYTransform 0.0)
                (else
                  (LocalVariables|SetnewYTransform -2e+02) ; Background
                ))
              (Transformation|SetRelativeLocation _array_element_2 (Math|Vector|MakeVector (LocalVariables|GetnewYTransform) (.Y (Math|Vector|BreakVector (Variables|/Script/Engine.SceneComponent|GetRelativeLocation _array_element_2))) (.Z (Math|Vector|BreakVector (Variables|/Script/Engine.SceneComponent|GetRelativeLocation _array_element_2)))) false false))))
        (elif (Variables|Input|GetinputRight)
          (Math|Integer|IncrementInt (Variables|Default|GetplayerCommandGroup)
            (:%20%20
              (goto _label_2)))
          (else
            ;[1 1 1] Press A to select command group
            (if (Variables|Input|GetinputA)
              (commands|ToggleGroupBillboards)
              (commands|ToggleSubmenuText)
              (Variables|Default|SetinSubMenu true)
              (commands|GetCommandNames))))))))

(fn InputLag
  (params (dt :type Float%20%28single-precision%29))
  (if (Math|Boolean|ORBoolean (Variables|Input|GetinputRight) (Variables|Input|GetinputLeft) (Variables|Input|GetinputDown) (Variables|Input|GetinputUp))
    (if (<= (Variables|Default|GetdirectionInputLag) 0.0)
      (Variables|Default|SetdirectionInputLag 0.25)
      (Variables|Input|SetinputRight false :!label _label)
      (Variables|Input|SetinputLeft false)
      (Variables|Input|SetinputDown false)
      (Variables|Input|SetinputUp false))
    (elif (> (Variables|Default|GetdirectionInputLag) 0.0)
      (Variables|Default|SetdirectionInputLag (- (Variables|Default|GetdirectionInputLag) (* dt (Math|Float|MakeLiteralFloat 1.0))))
      (goto _label))))

(fn ToggleGroupBillboards
  ;[1 1 1] Disable command group objects
  (for _array_element (Variables|Default|GetcommandGroupBillboards)
    (Rendering|ToggleVisibility _array_element false)))

(fn ToggleSubmenuText
  ;[1 1 1] Enable submenu objects
  (for _array_element (Variables|Default|GetcommandTexts)
    (Rendering|ToggleVisibility _array_element true)))

(fn CreateTarget
  (params (targets :type Integer))
  (bind _output_get (LocalVariables|SettargetType targets))
  (if (== _output_get (Class|KismetMathLibrary|OrIntInt 2 3)) ; All foes?
    (for _array_element (Variables|enemies|Getenemeies)
      (if (== (LocalVariables|GettargetType) 2) ; Attack all or attack all grounded enemies?
        (if (Variables|/Game/Blueprints/Blueprints/Enemies/BP_EnemyBattler.BP_EnemyBattler_C|Getgrounded _array_element) ; If ignoring air enemies they don't get a target
          (bind _returnvalue (Game|SpawnActorfromClass "/Game/Blueprints/Blueprints/BP_TargetSelector.BP_TargetSelector_C" (Transformation|GetActorTransform _array_element) "AlwaysSpawn" 0 0 :!label _label))
          (Variables|/Game/Blueprints/Blueprints/BP_TargetSelector.BP_TargetSelector_C|Settype _returnvalue (LocalVariables|GettargetType)))
        (else
          (goto _label))))
    (elif (== (LocalVariables|GettargetType) 5) ; All allies?
      (for _array_element_2 (Variables|Default|Getallies)
        (bind _returnvalue_2 (Game|SpawnActorfromClass "/Game/Blueprints/Blueprints/BP_TargetSelector.BP_TargetSelector_C" (Transformation|GetActorTransform _array_element_2) "AlwaysSpawn" 0 0))
        (Variables|/Game/Blueprints/Blueprints/BP_TargetSelector.BP_TargetSelector_C|Settype _returnvalue_2 (LocalVariables|GettargetType)))
      (elif (== (LocalVariables|GettargetType) 5) ; Singly ally?
        (bind _returnvalue_3 (Game|SpawnActorfromClass "/Game/Blueprints/Blueprints/BP_TargetSelector.BP_TargetSelector_C" (Transformation|GetActorTransform (Utilities|Array|Get(acopy) (Variables|Default|Getallies))) "Undefined" 0 0))
        (Variables|/Game/Blueprints/Blueprints/BP_TargetSelector.BP_TargetSelector_C|Settype _returnvalue_3 (LocalVariables|GettargetType))
        (else
          (bind _returnvalue_4 (Game|SpawnActorfromClass "/Game/Blueprints/Blueprints/BP_TargetSelector.BP_TargetSelector_C" (Transformation|GetActorTransform (Utilities|Array|Get(acopy) (Variables|enemies|Getenemeies))) "Undefined" 0 0)) ; Single foe
          (Variables|/Game/Blueprints/Blueprints/BP_TargetSelector.BP_TargetSelector_C|Settype _returnvalue_4 (LocalVariables|GettargetType)))))))

(fn SelectTarget
  (if (not (Variables|playerActions|GetactionCommandOccuring))
    (if (Variables|Input|GetinputRight)
      (Math|Integer|IncrementInt (Variables|Default|GetselectedTarget)
        (:%20%20
          (Variables|Default|SetselectedTarget (Math|Integer|Clamp(Integer) (Variables|Default|GetselectedTarget) 0 (- (Utilities|Array|Length (Variables|enemies|Getenemeies)) 1)) :!label _label)))
      (elif (Variables|Input|GetinputLeft)
        (Math|Integer|DecrementInt (Variables|Default|GetselectedTarget)
          (:%20%20
            (goto _label)))
        (else
          ;[1 1 1] Press A to proceed to fight target
          (if (Variables|Input|GetinputA)
            (Variables|Default|Setmode "NewEnumerator4")
            (Variables|playerActions|SetactionCommandOccuring true)
            (BattleAction|CreateActionActor)
            ;[1 1 1] Remove targets
            (bind _outactors (Actor|GetAllActorsOfClass "/Game/Blueprints/Blueprints/BP_TargetSelector.BP_TargetSelector_C" :!label _label_2))
            (bind _arrayelement (Utilities|Array|ReverseforEachLoop _outactors)
              (:LoopBody
                (Actor|DestroyActor _arrayelement)))
            (else
              ;[1 1 1] Press B to back out
              (if (Variables|Input|GetinputB)
                (commands|ToggleSubmenuText)
                (Variables|Default|Setmode "NewEnumerator0")
                (goto _label_2)))))))))

(fn PlayerAttacking
  (params (target :type Integer) (attackName :type String) (badgeStatus :type Integer) (badgeElement :type Integer) (actionCommandRating :type Integer))
  (bind _gamemode (Variables|Default|GetgameMode))
  (bind _enemeies (Variables|enemies|Getenemeies))
  (bind _selectedtarget (Variables|Default|GetselectedTarget))
  (bind _output (Utilities|Array|Get(acopy) _enemeies _selectedtarget))
  ;[1 1 1] Get actor for damage function (should prob make this a variable)
  (bind _outactors (Actor|GetAllActorsOfClass "/Game/Blueprints/Blueprints/Character/BP_AllyBattler.BP_AllyBattler_C"))
  (LocalVariables|SetallyBattler (Utilities|Array|Get(acopy) _outactors))
  (LocalVariables|SetactionRating actionCommandRating)
  (Variables|/Game/Blueprints/Blueprints/RPG_GameMode.RPG_GameMode_C|SetMP _gamemode (- (Variables|/Game/Blueprints/Blueprints/RPG_GameMode.RPG_GameMode_C|GetMP _gamemode) (.mpCost (Utilities|Struct|BreakSt_AttacksAndAbilities (Variables|Default|GetcurrentPlayerAttack)))))
  (LocalVariables|SetplayerDamage (+ (* 0 1) (LocalVariables|GetactionRating)))
  ;[1 1 1] Damage Enemy
  (bind (_newhp _outputdamage) (Default|CalculateDamage (LocalVariables|GetallyBattler) (LocalVariables|GetplayerDamage) 0 (Variables|/Game/Blueprints/Blueprints/Enemies/BP_EnemyBattler.BP_EnemyBattler_C|GetHP _output) (Variables|/Game/Blueprints/Blueprints/Enemies/BP_EnemyBattler.BP_EnemyBattler_C|GetDef _output) true))
  (Variables|/Game/Blueprints/Blueprints/Enemies/BP_EnemyBattler.BP_EnemyBattler_C|SetHP _output _newhp)
  (Default|UpdateHPBar _output)
  ;[1 1 1] Output damage text
  (bind _returnvalue (Game|SpawnActorfromClass "/Game/Blueprints/Blueprints/BP_splashDamage.BP_splashDamage_C" (Math|Transform|MakeTransform (+ (Transformation|GetActorLocation (Utilities|Array|Get(acopy) (Variables|enemies|Getenemeies) (Variables|Default|GetselectedTarget))) "10.000000,10.000000,100.000000") "0, 0, 0" "2.000000,2.000000,2.000000") "Undefined" 0 0))
  (Rendering|Components|TextRender|SetText (Variables|/Game/Blueprints/Blueprints/BP_splashDamage.BP_splashDamage_C|GetTextRender _returnvalue) (Utilities|Text|ToText(Integer) _outputdamage))
  (BattleAction|PlayerEndingTurn))

(fn CreateActionActor
  (switch int (Variables|Default|Getsubmenu) ; What type of command is it?
    (:Default
      _)
    (:0
      _))
  ;[1 1 1] Using a badge (including default attacks)
  (bind _asrpg_game_mode (Utilities|Casting|CastToRPG_GameMode (Game|GetGameMode)))
  (Game|SpawnActorfromClass (Utilities|Array|Get(acopy) (Variables|playerActions|GetactionClasses) (.badgeID (Utilities|Struct|BreakSt_Badges (Utilities|Array|Get(acopy) (Variables|/Game/Blueprints/Blueprints/RPG_GameMode.RPG_GameMode_C|GetbadgeInventory _asrpg_game_mode) (Variables|Default|GetcommandSelected))))) (Transformation|GetActorTransform) "Undefined" 0 0))

(fn GetCommandNames
  (bind _gamemode (Variables|Default|GetgameMode))
  (switch int (Variables|Default|Getsubmenu) ; 0 = Attacks, 1 = Items, 2 = Tactics
    (:0
      (if (Variables|playerActions|GetcurrentTurnOfPartner) ; Partners have their own specific attacks...
        ;[1 1 1] Make every menu item into a partner attack command
        (for (_array_element _array_index) (.attackNames (Utilities|Struct|BreakSt_Partners (Utilities|Array|Get(acopy) (Variables|/Game/Blueprints/Blueprints/RPG_GameMode.RPG_GameMode_C|GetpartnersInParty _gamemode) (Variables|/Game/Blueprints/Blueprints/RPG_GameMode.RPG_GameMode_C|GetcurrentPartner _gamemode))))
          (if (.ReturnValue (Utilities|Map|Find (Variables|/Game/Blueprints/Blueprints/RPG_GameMode.RPG_GameMode_C|GetDB_PartnerAbilities (Variables|Default|GetgameMode)) _array_element))
            (Rendering|Components|TextRender|SetText (Utilities|Array|Get(acopy) (Variables|Default|GetcommandTexts) _array_index) (Utilities|Text|ToText(String) _array_element))
            ;[1 1 1] MP Cost Text
            (bind _astext_render_component (Utilities|Casting|CastToTextRenderComponent (Components|GetChildComponent (Utilities|Array|Get(acopy) (Variables|Default|GetcommandTexts) _array_index) 0)))
            (Rendering|Components|TextRender|SetText _astext_render_component (Utilities|Text|ToText(Integer) (.mpCost (Utilities|Struct|BreakSt_AttacksAndAbilities (.Value (Utilities|Map|Find (Variables|/Game/Blueprints/Blueprints/RPG_GameMode.RPG_GameMode_C|GetDB_PartnerAbilities (Variables|Default|GetgameMode)) _array_element))))))))
        (else
          ;[1 1 1] Make every menu item into an attack command (Based on equipped badges that are attacks)
          (for (_array_element_2 _array_index_2) (Variables|/Game/Blueprints/Blueprints/RPG_GameMode.RPG_GameMode_C|GetbadgeInventory (Variables|Default|GetgameMode))
            (if (.isAbility (Utilities|Struct|BreakSt_Badges _array_element_2))
              (Rendering|Components|TextRender|SetText (Utilities|Array|Get(acopy) (Variables|Default|GetcommandTexts) _array_index_2) (.Name (Utilities|Struct|BreakSt_Badges _array_element_2)))
              ;[1 1 1] MP Cost Text
              (bind _astext_render_component_2 (Utilities|Casting|CastToTextRenderComponent (Components|GetChildComponent (Utilities|Array|Get(acopy) (Variables|Default|GetcommandTexts) _array_index_2) 0)))
              (Rendering|Components|TextRender|SetText _astext_render_component_2 (Utilities|Text|ToText(Integer) (.mpCost (Utilities|Struct|BreakSt_Badges _array_element_2)))))))))))

(fn StartEnemyTurn
  (if (not (Variables|enemies|GetwaitingOnEnemy))
    (Variables|Input|SetinputA false)
    (Variables|Input|SetinputB false)
    (Default|PickCommand (Utilities|Array|Get(acopy) (Variables|enemies|Getenemeies) (Variables|enemies|GetenemyTurnIndex)))
    (Variables|enemies|SetwaitingOnEnemy true)))

(fn EndEnemyTurn
  (bind _result (Math|Integer|IncrementInt (Variables|enemies|GetenemyTurnIndex))
    (:%20%20
      (Variables|enemies|SetwaitingOnEnemy false)
      ;[1 1 1] Check if there's more enemies waiting for their turn
      (if (>= _result (Utilities|Array|Length (Variables|enemies|Getenemeies)))
        (Variables|Default|Setmode "NewEnumerator3")
        (Variables|enemies|SetenemyTurnIndex 0)))))

(fn EndTurn
  (Variables|Default|Setmode "NewEnumerator0")
  (Variables|playerActions|SetcurrentTurnOfPartner false) ; Change this if partner set to be in front
  (commands|ToggleGroupBillboards)
  (Variables|Default|SetbriefDelay true))

(fn PlayerEndingTurn
  ;[1 1 1] Check if everyone has gone yet, if so it's the enemies' turn.
  (Variables|Default|SetinSubMenu false)
  (Variables|playerActions|SetactionCommandOccuring false)
  (if (Variables|playerActions|GetcurrentTurnOfPartner)
    (Variables|playerActions|SetpartnerTookTurn true)
    (if (Variables|playerActions|GetpartnerTookTurn)
      (Variables|Default|Setmode "NewEnumerator2" :!label _label)
      (Variables|playerActions|SetplayerTookTurn false)
      (Variables|playerActions|SetpartnerTookTurn false)
      (Variables|Default|SetbriefDelay true)
      (else
        (Variables|playerActions|SetcurrentTurnOfPartner false)
        (Variables|Default|Setmode "NewEnumerator0" :!label _label_2)
        (commands|ToggleGroupBillboards)))
    (else
      (Variables|playerActions|SetplayerTookTurn true)
      (if (Variables|playerActions|GetpartnerTookTurn)
        (goto _label)
        (else
          (Variables|playerActions|SetcurrentTurnOfPartner true)
          (goto _label_2))))))